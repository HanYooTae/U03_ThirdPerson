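; BP_Door is a double sliding door that opens when a Character overlaps it and closes when the overlap ends.
; One timeline, played and reversed, slides both panels in opposite directions and rotates the lock.
; A dynamic material from the construction script turns the lock's emissive green on entry and red once fully closed.
; Any overlapping actor shows and recolors the point light, and ending overlap hides it.
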(event `self.ReceiveActorBeginOverlap`
  (params (OtherActor :type "Actor Object Reference"))
  (`SceneComponent.SetVisibility` (`self.PointLight`) true false)
  (`LightComponent.SetLightColor` (`self.PointLight`) (`self.OverlapColor`) true)
  (cast `Character` OtherActor)
  (`MaterialInstanceDynamic.SetVectorParameterValue` (`self.DynamicMaterial`) "Emissive" (make `LinearColor` 0.0 20.0))
  (bind (_direction _doorlocation _lockrotation) (`Timeline|DoorTimeline` :!label _label) ; 문 열리고 닫히는 이벤트
    (:`Update`
      (`|ExecutionSequence`
        (:`then_0`
          (bind _returnvalue (`KismetMathLibrary.MakeVector` 0.0 _doorlocation))
          (`SceneComponent.K2_SetRelativeLocation` (`self.RightDoor`) _returnvalue false false)
          (`SceneComponent.K2_SetRelativeLocation` (`self.LeftDoor`) (* _returnvalue -1.0) false false))
        (:`then_1`
          (`SceneComponent.K2_SetRelativeRotation` (`self.DoorLock`) (`KismetMathLibrary.MakeRotator` _lockrotation) false false))))
    (:`Finished`
      (if (`|EnumEquality` _direction "Backward")
        (`MaterialInstanceDynamic.SetVectorParameterValue` (`self.DynamicMaterial`) "Emissive" (make `LinearColor` 20.0))))))

(event `self.ReceiveActorEndOverlap`
  (params (OtherActor :type "Actor Object Reference"))
  (`SceneComponent.SetVisibility` (`self.PointLight`) false false)
  (cast `Character` OtherActor)
  (goto _label :!via `Reverse`))

(fn `UserConstructionScript`
  (bind _returnvalue (`KismetMaterialLibrary.CreateDynamicMaterialInstance` "/Game/Door/MAT_DoorLock_Inst.MAT_DoorLock_Inst"))
  (bind _output_get (set `self.DynamicMaterial` _returnvalue))
  (`PrimitiveComponent.SetMaterial` (`self.DoorLock`) 0 _output_get)
  (`LightComponent.SetLightColor` (`self.PointLight`) (`self.StartColor`) true))