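; Warp skill for the magic weapon system that teleports the owning character to the world-static surface under the cursor.
; While selected, Tick aligns a decal to the cursor trace hit, hiding the actor when nothing is hit.
; Spell stores a valid target, disables movement, plays a montage and launches the character upward.
; DoWarp then moves the character there with sweep, offset by capsule half-height, and EndSpell restores movement.
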(event `self.ReceiveBeginPlay`
  (`parent.ReceiveBeginPlay`)
  (`SceneComponent.SetVisibility` (`self.Decal`) false false))

(event `self.Spell`
  (bind _ascharacter (`self.GetOwnerToCharacter`))
  (`parent.Spell`)
  (bind _location (`self.GetCursorLocation`)
    (:`True`
      (set `self.WarpLocation` _location)
      (set `self.bCanWarp` true)
      (`/Game/Weapons/BP_Weapon.SetStateMove` (`self.GetOwnerToMagic`) false)
      (`Character.PlayAnimMontage` _ascharacter "/Game/Character/Montages/Magic/MG_Warp_Montage.MG_Warp_Montage" 1.0 "None")
      (`Character.LaunchCharacter` _ascharacter (0.0 0.0 500.0) false false))
    (:`False`
      (set `self.bCanWarp` false))))

(event `DoWarp`
  (bind _ascharacter (`self.GetOwnerToCharacter`))
  (bind (_warplocation_x _warplocation_y _warplocation_z) (`KismetMathLibrary.BreakVector` (`self.WarpLocation`)))
  (if (`self.bCanWarp`)
    (set `self.bCanWarp` false)
    (`self.K2_SetActorLocation` _ascharacter (`KismetMathLibrary.MakeVector` _warplocation_x _warplocation_y (+ (`CapsuleComponent.GetScaledCapsuleHalfHeight` (`Character.CapsuleComponent` _ascharacter)) _warplocation_z)) true false)))

(event `self.EndSpell`
  (`parent.EndSpell`)
  (`/Game/Weapons/BP_Weapon.SetStateMove` (`self.GetOwnerToMagic`) true))

(event `self.ReceiveTick`
  (params (DeltaSeconds :type "Float (single-precision)"))
  (if (`self.bEnabled`)
    (bind (_location _impactnormal) (`self.GetCursorLocation`)
      (:`True`
        (`SceneComponent.K2_SetWorldLocation` (`self.Decal`) _location false false)
        (`SceneComponent.K2_SetWorldRotation` (`self.Decal`) (`KismetMathLibrary.Conv_VectorToRotator` _impactnormal) false false))
      (:`False`
        (`self.SetActorHiddenInGame` true)))))

(event `self.OnSelect`
  (`parent.OnSelect`)
  (set `self.bEnabled` true)
  (`SceneComponent.SetVisibility` (`self.Decal`) true false))

(event `self.OffSelect`
  (`parent.OffSelect`)
  (set `self.bEnabled` false)
  (`SceneComponent.SetVisibility` (`self.Decal`) false false))

(fn `UserConstructionScript`
  (`parent.UserConstructionScript`))