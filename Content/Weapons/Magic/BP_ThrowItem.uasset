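; BP_ThrowItem is a thrown magic item that expires two seconds after spawning and delivers impact damage.
; It resolves its owner chain through BP_Skill_Throw to BP_Magic and the caster.
; SendDamage ignores the caster, spawns an impact emitter oriented along the caster-to-target direction, forwards damage on Characters to BP_Magic, then destroys the item.
; No movement or collision event appears here, and nothing in this graph calls SendDamage.
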(event `self.ReceiveBeginPlay`
  (`self.SetLifeSpan` 2.0))

(fn `GetOwnerToMagic`
  (returns (`AsBP Magic` :type "/Game/Weapons/Magic/BP_Magic Object Reference"))
  (bind _asbp_magic (cast `/Game/Weapons/Magic/BP_Magic` (`self.GetOwner` (`self.GetOwnerToThrow`))))
  (return _asbp_magic))

(fn `GetOwnerToThrow`
  (returns (`AsBP Skill Throw` :type "/Game/Weapons/Magic/BP_Skill_Throw Object Reference"))
  (bind _asbp_skill_throw (cast `/Game/Weapons/Magic/BP_Skill_Throw` (`self.GetOwner`)))
  (return _asbp_skill_throw))

(fn `Send Damage`
  (params (OtherActor :type "Actor Object Reference") (ImpactParticle :type "ParticleSystem Object Reference") (ImpactScale :type "Vector Structure" :default (1.0 1.0 1.0)) (Damage :type "Float (double-precision)" :default 1.0))
  (bind _returnvalue (`self.GetOwner` (`self.GetOwnerToMagic`)))
  (if (!= OtherActor _returnvalue)
    (`GameplayStatics.SpawnEmitterAtLocation` (`local.ImpactParticle`) (`self.K2_GetActorLocation`) (`KismetMathLibrary.FindLookAtRotation` (`self.K2_GetActorLocation` _returnvalue) (`self.K2_GetActorLocation` (`local.OtherActor`))) (`local.ImpactScale`))
    (cast `Character` (`local.OtherActor`)
      (:`then`
        (`/Game/Weapons/BP_Weapon.SendDamage` (`self.GetOwnerToMagic`) (`local.OtherActor`) (`local.Damage`)))
      (:`CastFailed`
        _))
    (`self.K2_DestroyActor`)))

(fn `UserConstructionScript`)