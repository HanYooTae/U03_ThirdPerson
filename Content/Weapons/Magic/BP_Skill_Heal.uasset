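; BP_Skill_Heal is a magic skill that heals the casting player.
; On cast it disables movement through the owner's magic interface or component, plays a buff montage on the character, and raises health by a fixed amount through the player's StatusComponent.
; The health gain applies immediately and only when the owner is a BP_Player.
; Ending the spell restores movement.
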(event `self.Spell`
  (`parent.Spell`)
  (`/Game/Weapons/BP_Weapon.SetStateMove` (`self.GetOwnerToMagic`) false)
  (`Character.PlayAnimMontage` (`self.GetOwnerToCharacter`) "/Game/Character/Montages/Magic/MG_Buff_Montage.MG_Buff_Montage" 1.0 "None")
  (bind _asbp_player (cast `/Game/Player/BP_Player` (`self.GetOwnerToCharacter`)))
  (`/Game/Components/StatusComponent.IncreaseHealth` (`/Game/Player/BP_Player.StatusComponent` _asbp_player) 10.0))

(event `self.EndSpell`
  (`parent.EndSpell`)
  (`/Game/Weapons/BP_Weapon.SetStateMove` (`self.GetOwnerToMagic`) true))

(fn `UserConstructionScript`
  (`parent.UserConstructionScript`))