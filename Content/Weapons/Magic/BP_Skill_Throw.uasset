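; BP_Skill_Throw is a magic skill that throws the currently selected item class from the character's hand.
; Selecting it shows that item's hand particle and puts BP_Player into aim; deselecting reverses both.
; Spell plays the fireball montage, while a separate DoThrow event spawns the projectile at the Hand_Throw socket, facing the control rotation.
; SetCurrentItem looks up a class in ThrowItems to update the selection and hand particle.
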(event `self.ReceiveBeginPlay`
  (bind (_output_throwitemclass _output_attachparticle) (break `/Game/Structs/FThrowItem` (`|GetArrayItem` (`self.ThrowItems`) (`self.Select`))))
  (`parent.ReceiveBeginPlay`)
  (`ParticleSystemComponent.SetTemplate` (`self.HandParticle`) _output_attachparticle)
  (`SceneComponent.SetVisibility` (`self.HandParticle`) false false))

(event `self.Spell`
  (`parent.Spell`)
  (`Character.PlayAnimMontage` (`self.GetOwnerToCharacter`) "/Game/Character/Montages/Magic/MG_Fireball_03_Montage.MG_Fireball_03_Montage" 1.0 "None"))

(event `DoThrow`
  (bind _output_throwitemclass (break `/Game/Structs/FThrowItem` (`|GetArrayItem` (`self.ThrowItems`) (`self.Select`))))
  (`|SpawnActorFromClass` _output_throwitemclass (`KismetMathLibrary.MakeTransform` (`SceneComponent.GetSocketLocation` (`Character.Mesh` (`self.GetOwnerToCharacter`)) "Hand_Throw") (`Controller.GetControlRotation` (`GameplayStatics.GetPlayerController` 0))) "Undefined" "OverrideRootScale" self null))

(event `self.EndSpell`
  (`parent.EndSpell`))

(event `self.OnSelect`
  (`parent.OnSelect`)
  (`SceneComponent.SetVisibility` (`self.HandParticle`) true false)
  (bind _asbp_player (cast `/Game/Player/BP_Player` (`self.GetOwnerToCharacter`)))
  (`/Game/Player/BP_Player.OnAim` _asbp_player))

(event `self.OffSelect`
  (`parent.OffSelect`)
  (`SceneComponent.SetVisibility` (`self.HandParticle`) false false)
  (bind _asbp_player (cast `/Game/Player/BP_Player` (`self.GetOwnerToCharacter`)))
  (`/Game/Player/BP_Player.OffAim` _asbp_player))

(fn `SetCurrentItem`
  (params (ThrowItemClass :type "/Game/Weapons/Magic/BP_ThrowItem Class Reference"))
  (locals (Iterator :type Integer))
  (bind (_output_throwitemclass _output_attachparticle) (break `/Game/Structs/FThrowItem` (`|GetArrayItem` (`self.ThrowItems`) (`local.Iterator`))))
  (bind _output_throwitemclass_2 (break `/Game/Structs/FThrowItem` (`|GetArrayItem` (`self.ThrowItems`) (`local.Iterator`))))
  (for (_ _array_index) (`self.ThrowItems`)
    (set `local.Iterator` _array_index)
    (if (== _output_throwitemclass_2 (`local.ThrowItemClass`))
      (break)))
  (set `self.Select` (`local.Iterator`))
  (`ParticleSystemComponent.SetTemplate` (`self.HandParticle`) _output_attachparticle))

(fn `UserConstructionScript`
  (`parent.UserConstructionScript`))