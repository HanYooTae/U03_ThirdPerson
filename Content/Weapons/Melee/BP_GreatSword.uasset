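; BP_GreatSword is a melee greatsword Blueprint that extends a parent weapon class with capsule-based hit detection.
; The parent's collision events toggle the capsule, whose overlaps pass DamageComponent's single-hit damage to SendDamage.
; Critical start and end events forward to DamageComponent, with the combo count on start.
; The SendDamage override ignores that damage, doing nothing for BP_Enemy and calling the parent with zero damage when the cast fails.
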(event `self.ReceiveBeginPlay`
  (`parent.ReceiveBeginPlay`)
  (`PrimitiveComponent.SetCollisionEnabled` (`self.Capsule`) "NoCollision"))

(event `self.OnCollision`
  (params (SpecificCollision :type "/Game/Enum/ECollisionType Enum" :default "NewEnumerator0"))
  (`parent.OnCollision` SpecificCollision)
  (`PrimitiveComponent.SetCollisionEnabled` (`self.Capsule`) "QueryAndPhysics"))

(event `self.OffCollision`
  (`parent.OffCollision`)
  (`PrimitiveComponent.SetCollisionEnabled` (`self.Capsule`) "NoCollision"))

(event `self.Capsule.OnComponentBeginOverlap`
  (params (OverlappedComponent :type "PrimitiveComponent Object Reference") (OtherActor :type "Actor Object Reference") (OtherComp :type "PrimitiveComponent Object Reference") (OtherBodyIndex :type Integer) (bFromSweep :type Boolean) (SweepResult :type "HitResult Structure (by ref)"))
  (bind _returnvalue (`/Game/Components/DamageComponent.GetSingleDamage` (`self.DamageComponent`)))
  (`self.SendDamage` OtherActor _returnvalue))

(event `self.StartCritical`
  (`parent.StartCritical`)
  (`/Game/Components/DamageComponent.StartCritical` (`self.DamageComponent`) (`self.ComboCount`)))

(event `self.EndCritical`
  (`parent.EndCritical`)
  (`/Game/Components/DamageComponent.EndCritical` (`self.DamageComponent`)))

(fn `SendDamage`
  (params (OtherActor :type "Actor Object Reference") (Damage :type "Float (double-precision)"))
  (returns (Result :type Boolean))
  (bind _asbp_enemy (cast `/Game/Enemies/BP_Enemy` OtherActor)
    (:`CastFailed`
      (bind _result (`parent.SendDamage` _asbp_enemy 0.0))
      (return _result))))

(fn `UserConstructionScript`)