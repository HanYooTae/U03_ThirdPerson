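; Base melee weapon that runs data-driven combo attacks, with collision and critical hooks for child weapons.
; BeginPlay gathers data table rows matching its melee type; each supplies a combo step's montage and movement permission.
; Attack input during the combo window queues the next step, which NextCombo plays until EndAttack resets everything.
; SendDamage filters already-hit actors, then successful hits trigger camera shake and brief slow-motion hit-stop, plus lightning on the last combo.
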(event `self.ReceiveBeginPlay`
  ;[1 1 1] Read Data Table
  (`parent.ReceiveBeginPlay`)
  (bind _outrownames (`DataTableFunctionLibrary.GetDataTableRowNames` (`self.DataTable`)))
  (for _array_element _outrownames
    (bind _returnvalue (`|GetDataTableRow` (`self.DataTable`) _array_element)
      (:`then`
        (if (`|EnumEquality` (`.Type_18_9CFC950948CD2F5E840C3D979CAC5252` (break `/Game/Structs/FMeleeData` _returnvalue)) (`self.MeleeType`))
          (`KismetArrayLibrary.Array_Add` (`self.MeleeDatas`) _returnvalue))))))

(event `self.Attack`
  ;[1 1 1] Attack(마우스 왼쪽 클릭)
  (`parent.Attack`)
  (if (`self.bCanCombo`)
    (set `self.bCanCombo` false)
    (set `self.bSucceedCombo` true)
    (elif (`self.CanAttack`)
      (`self.SetStateAttacking`)
      (`self.PlayComboMontage`)
      (`self.StartCritical`))))

(event `NextCombo`
  ;[1 1 1] 콤보 연결 성공 시
  (if (`self.bSucceedCombo`)
    (set `self.bSucceedCombo` false)
    (`/Engine/EditorBlueprintResources/StandardMacros.IncrementInt` (`self.ComboCount`)
      (:`  `
        (`self.PlayComboMontage`)
        (set `self.bLastCombo` (== (`self.ComboCount`) (- (`KismetArrayLibrary.Array_Length` (`self.MeleeDatas`)) 1)))))))

(event `self.EndAttack`
  ;[1 1 1] 공격 종료(콤보가 연결 실패거나 막타인 경우)
  (`parent.EndAttack`)
  (`self.SetStateIdling`)
  (`self.SetStateMove` true)
  (set `self.ComboCount` 0)
  (set `self.bSucceedCombo` false)
  (set `self.bLastCombo` false)
  (`self.EndCritical`))

(event `DamageEffect`
  ;[1 1 1] 타격 효과
  (if (`self.bLastCombo`)
    (`GameplayStatics.SpawnEmitterAtLocation` "/Game/InfinityBladeEffects/Effects/FX_Monsters/FX_Monster_Genno/P_Genno_Weapon_Lightning_01.P_Genno_Weapon_Lightning_01" (`self.K2_GetActorLocation`)))
  (`PlayerCameraManager.PlayCameraShake` :`self` (`PlayerController.PlayerCameraManager` (`GameplayStatics.GetPlayerController` 0)) :`ShakeClass` "/Game/Weapons/BP_MeleeShake.BP_MeleeShake_C")
  (`GameplayStatics.SetGlobalTimeDilation` 0.15)
  (`KismetSystemLibrary.Delay` 0.1)
  (`GameplayStatics.SetGlobalTimeDilation` 1.0))

(fn `EndCritical`)

(fn `OffCollision`
  (`KismetArrayLibrary.Array_Clear` (`self.HittedActors`)))

(fn `OnCollision`
  (params (SpecificCollision :type "/Game/Enum/ECollisionType Enum" :default "NewEnumerator0")))

(fn `PlayComboMontage`
  (bind (_output_type _output_montage _output_playrate _output_sectionname _output_bcanmove) (break `/Game/Structs/FMeleeData` (`|GetArrayItem` (`self.MeleeDatas`) (`self.ComboCount`))))
  (bind _ascharacter (cast `Character` (`self.GetOwner`)))
  (`Character.PlayAnimMontage` _ascharacter _output_montage _output_playrate _output_sectionname)
  (`self.SetStateMove` _output_bcanmove))

(fn `SendDamage`
  (params (OtherActor :type "Actor Object Reference") (Damage :type "Float (double-precision)"))
  (returns (Result :type Boolean))
  (locals (bDuplicateActors :type Boolean))
  (for _array_element (`self.HittedActors`)
    (if (== _array_element (`local.OtherActor`))
      (set `local.bDuplicateActors` true)
      (break)))
  (if (not (`local.bDuplicateActors`))
    (`KismetArrayLibrary.Array_Add` (`self.HittedActors`) (`local.OtherActor`))
    (bind _result (`parent.SendDamage` (`local.OtherActor`) (`local.Damage`)))
    (if _result
      (`self.DamageEffect`)
      (return _result)
      (else
        (return false)))))

(fn `StartCritical`)

(fn `UserConstructionScript`
  (`parent.UserConstructionScript`))