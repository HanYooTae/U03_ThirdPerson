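; BP_Fist is an unarmed melee weapon with four hit volumes for left and right punches and kicks.
; On BeginPlay it attaches each volume to the owner character's mesh socket of the same name and disables collision.
; OnCollision enables the requested limb's volume and OffCollision disables all spheres.
; Overlaps send combo-count-based damage from DamageComponent, which also receives critical start and end calls.
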(event `self.ReceiveBeginPlay`
  (`parent.ReceiveBeginPlay`)
  (`self.AttachCollisionToSocket` (`self.LeftPunch`))
  (`self.AttachCollisionToSocket` (`self.RightPunch`))
  (`self.AttachCollisionToSocket` (`self.LeftKick`))
  (`self.AttachCollisionToSocket` (`self.RightKick`))
  (`self.SetAllCollisions` "NoCollision"))

(event `self.OnCollision`
  (params (SpecificCollision :type "/Game/Enum/ECollisionType Enum" :default "NewEnumerator0"))
  (`parent.OnCollision` SpecificCollision)
  (switch `/Game/Enum/ECollisionType` SpecificCollision
    (:`NewEnumerator1`
      (`PrimitiveComponent.SetCollisionEnabled` (`self.LeftPunch`) "QueryAndPhysics"))
    (:`NewEnumerator2`
      (`PrimitiveComponent.SetCollisionEnabled` (`self.RightPunch`) "QueryAndPhysics"))
    (:`NewEnumerator3`
      (`PrimitiveComponent.SetCollisionEnabled` (`self.LeftKick`) "QueryAndPhysics"))
    (:`NewEnumerator4`
      (`PrimitiveComponent.SetCollisionEnabled` (`self.RightKick`) "QueryAndPhysics"))))

(event `self.OffCollision`
  (`parent.OffCollision`)
  (`self.SetAllCollisions` "NoCollision"))

(event `self.LeftPunch.OnComponentBeginOverlap`
  (params (OverlappedComponent :type "PrimitiveComponent Object Reference") (OtherActor :type "Actor Object Reference") (OtherComp :type "PrimitiveComponent Object Reference") (OtherBodyIndex :type Integer) (bFromSweep :type Boolean) (SweepResult :type "HitResult Structure (by ref)"))
  (bind _returnvalue (`/Game/Components/DamageComponent.GetComboDamage` (`self.DamageComponent`) (`self.ComboCount`)))
  (`self.SendDamage` OtherActor _returnvalue))

(event `self.RightPunch.OnComponentBeginOverlap`
  (params (OverlappedComponent :type "PrimitiveComponent Object Reference") (OtherActor :type "Actor Object Reference") (OtherComp :type "PrimitiveComponent Object Reference") (OtherBodyIndex :type Integer) (bFromSweep :type Boolean) (SweepResult :type "HitResult Structure (by ref)"))
  (bind _returnvalue (`/Game/Components/DamageComponent.GetComboDamage` (`self.DamageComponent`) (`self.ComboCount`)))
  (`self.SendDamage` OtherActor _returnvalue))

(event `self.LeftKick.OnComponentBeginOverlap`
  (params (OverlappedComponent :type "PrimitiveComponent Object Reference") (OtherActor :type "Actor Object Reference") (OtherComp :type "PrimitiveComponent Object Reference") (OtherBodyIndex :type Integer) (bFromSweep :type Boolean) (SweepResult :type "HitResult Structure (by ref)"))
  (bind _returnvalue (`/Game/Components/DamageComponent.GetComboDamage` (`self.DamageComponent`) (`self.ComboCount`)))
  (`self.SendDamage` OtherActor _returnvalue))

(event `self.RightKick.OnComponentBeginOverlap`
  (params (OverlappedComponent :type "PrimitiveComponent Object Reference") (OtherActor :type "Actor Object Reference") (OtherComp :type "PrimitiveComponent Object Reference") (OtherBodyIndex :type Integer) (bFromSweep :type Boolean) (SweepResult :type "HitResult Structure (by ref)"))
  (bind _returnvalue (`/Game/Components/DamageComponent.GetComboDamage` (`self.DamageComponent`) (`self.ComboCount`)))
  (`self.SendDamage` OtherActor _returnvalue))

(event `self.StartCritical`
  (`parent.StartCritical`)
  (`/Game/Components/DamageComponent.StartCritical` (`self.DamageComponent`) (`self.ComboCount`)))

(event `self.EndCritical`
  (`parent.EndCritical`)
  (`/Game/Components/DamageComponent.EndCritical` (`self.DamageComponent`)))

(fn `AttachCollisionToSocket`
  (params (InCollision :type "ShapeComponent Object Reference"))
  (bind _ascharacter (cast `Character` (`self.GetOwner`)))
  (`SceneComponent.K2_AttachToComponent` (`local.InCollision`) (`Character.Mesh` _ascharacter) (`KismetStringLibrary.Conv_StringToName` (`KismetSystemLibrary.GetObjectName` (`local.InCollision`))) "KeepRelative" "KeepRelative" "KeepRelative" true))

(fn `SetAllCollisions`
  (params (InCollisionType :type "ECollisionEnabled Enum" :default "NoCollision"))
  (for _array_element (`self.K2_GetComponentsByClass` "/Script/Engine.SphereComponent")
    (`PrimitiveComponent.SetCollisionEnabled` _array_element (`local.InCollisionType`))))

(fn `UserConstructionScript`)