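; BP_MovingTrigger2 is a Stage 1 trigger actor that signals overlaps with a point light and spawns the next trigger in a chain.
; The construction script applies the start color, and the light is visible from BeginPlay.
; Overlap switches it to the overlap color, with a DoOnce spawning BP_MovingTrigger3 at a fixed offset from this actor.
; Ending overlap hides the light; a call to destroy MovingTrigger1 is left unconnected.
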(event `self.ReceiveBeginPlay`
  (`SceneComponent.SetVisibility` (`self.PointLight`) true false))

(event `self.ReceiveActorBeginOverlap`
  (params (OtherActor :type "Actor Object Reference"))
  (`SceneComponent.SetVisibility` (`self.PointLight`) true false)
  (`LightComponent.SetLightColor` (`self.PointLight`) (`self.OverlapColor`) true)
  (`/Engine/EditorBlueprintResources/StandardMacros.DoOnce` false
    (:`Completed`
      (`|SpawnActorFromClass` "/Game/과제/Stage1/BP_MovingTrigger3.BP_MovingTrigger3_C" (`KismetMathLibrary.MakeTransform` (+ (`self.K2_GetActorLocation`) (500.0 250.0 0.0))) "Undefined" "OverrideRootScale" null null))))

(event `self.ReceiveActorEndOverlap`
  (params (OtherActor :type "Actor Object Reference"))
  (`SceneComponent.SetVisibility` (`self.PointLight`) false false))

(fn `UserConstructionScript`
  (`LightComponent.SetLightColor` (`self.PointLight`) (`self.StartColor`) true))