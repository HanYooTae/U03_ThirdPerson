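; Boss character that wields a spawned greatsword, reacts to damage and dies as a ragdoll.
; AnyDamage subtracts health, plays a hit montage, turns the boss toward its attacker and flashes red through dynamic materials.
; At zero health it ragdolls with a damage-scaled push away from the attacker, then destroys itself and the sword after a delay.
; State queries compare StateType, while the state setters are stubs returning false.
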(event `self.ReceiveBeginPlay`
  (`|ExecutionSequence`
    (:`then_0`
      (bind _returnvalue (`|SpawnActorFromClass` "/Game/Weapons/Melee/BP_GreatSword.BP_GreatSword_C" (`KismetMathLibrary.MakeTransform` (0.0 0.0 0.0)) "Undefined" "OverrideRootScale" self null))
      (bind _output_get (set `self.GreatSword` _returnvalue))
      (`self.K2_AttachToComponent` _output_get (`self.Mesh`) "Hand_GreateSword" "KeepRelative" "KeepRelative" "KeepRelative" true))))

(event `self.ReceiveAnyDamage`
  (params (Damage :type "Float (single-precision)") (DamageType :type "DamageType Object Reference") (InstigatedBy :type "Controller Object Reference") (DamageCauser :type "Actor Object Reference"))
  (set `self.Causer` DamageCauser) ; 데미지를 입힌 무기
  (bind _ascharacter (cast `Character` (`Controller.K2_GetPawn` InstigatedBy)))
  (set `self.Attacker` _ascharacter) ; 나를 때린 공격자
  (set `self.Damage` Damage)
  (set `self.Health` (- (`self.Health`) (`self.Damage`)))
  (`self.PlayAnimMontage` "/Game/Character/Montages/Common/HitReaction_Montage.HitReaction_Montage" 3.0)
  (`self.K2_SetActorRotation` (`KismetMathLibrary.FindLookAtRotation` (`self.K2_GetActorLocation`) (`self.K2_GetActorLocation` (`self.Attacker`))))
  (`self.ChangeBodyColor` (struct :`R` 1.0 :`A` 1.0))
  (`KismetSystemLibrary.Delay` 0.1)
  (`self.ChangeBodyColor` (struct :`R` 0.45098 :`G` 0.403922 :`B` 0.360784))
  (if (<= (`self.Health`) 0.0)
    (if (`|EnumInequality` (`self.StateType`) "NewEnumerator4")
      (set `self.StateType` "NewEnumerator4")
      (`self.Ragdoll`)
      (`self.Dead`))))

(event `Dead`
  (`KismetSystemLibrary.Delay` 5.0)
  (`self.K2_DestroyActor` (`self.GreatSword`))
  (`self.K2_DestroyActor`))

(fn `ChangeBodyColor`
  (params (NewColor :type "LinearColor Structure"))
  (for _array_element (`self.DynamicMaterials`)
    (`MaterialInstanceDynamic.SetVectorParameterValue` _array_element "BodyColor" (`local.NewColor`))))

(fn `IsStateAttacking`
  (returns (Result :type Boolean))
  (return (`|EnumEquality` (`self.StateType`) "NewEnumerator3")))

(fn `IsStateIdling`
  (returns (Result :type Boolean))
  (return (`|EnumEquality` (`self.StateType`) "NewEnumerator0")))

(fn `Ragdoll`
  (bind _mesh (`self.Mesh`))
  (set `SkeletalMeshComponent.GlobalAnimRateScale` 0.0 (`self.Mesh`))
  (`PrimitiveComponent.SetCollisionEnabled` (`self.CapsuleComponent`) "NoCollision")
  (`PrimitiveComponent.SetCollisionEnabled` _mesh "PhysicsOnly")
  (`PrimitiveComponent.SetSimulatePhysics` _mesh true)
  (`PrimitiveComponent.AddForce` (`self.Mesh`) (* (* (`KismetMathLibrary.GetDirectionUnitVector` (`self.K2_GetActorLocation` (`self.Attacker`)) (`self.K2_GetActorLocation`)) (`self.Damage`)) 250000.0) "None" false))

(fn `SetStateAttacking`
  (returns (Result :type Boolean))
  (return false))

(fn `SetStateIdling`
  (returns (Result :type Boolean))
  (return false))

(fn `SetStateMove`
  (params (bCanMove :type Boolean))
  (returns (Result :type Boolean))
  (return false))

(fn `SetStateSpelling`
  (returns (Result :type Boolean))
  (return false))

(fn `UserConstructionScript`
  (`|ExecutionSequence`
    (:`then_0`
      (bind _returnvalue (`KismetMaterialLibrary.CreateDynamicMaterialInstance` "/Game/Character/Materials/M_UE4Man_Body.M_UE4Man_Body"))
      (`KismetArrayLibrary.Array_Add` (`self.DynamicMaterials`) _returnvalue)
      (bind _returnvalue_2 (`KismetMaterialLibrary.CreateDynamicMaterialInstance` "/Game/Character/Materials/M_UE4Man_ChestLogo.M_UE4Man_ChestLogo"))
      (`KismetArrayLibrary.Array_Add` (`self.DynamicMaterials`) _returnvalue_2))
    (:`then_1`
      (`PrimitiveComponent.SetMaterial` (`self.Mesh`) 0 (`|GetArrayItem` (`self.DynamicMaterials`)))
      (`PrimitiveComponent.SetMaterial` (`self.Mesh`) 1 (`|GetArrayItem` (`self.DynamicMaterials`) 1)))))