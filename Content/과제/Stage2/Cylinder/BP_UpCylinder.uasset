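; BP_UpCylinder is a moving cylinder actor that oscillates between its placed location and a point 500 units along its up vector.
; On BeginPlay it caches both endpoints, then a timeline drives a location lerp without sweep.
; The timeline's Finished output feeds back into a FlipFlop that alternates Play and Reverse, so the motion loops indefinitely.
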(event `self.ReceiveBeginPlay`
  (bind _returnvalue (`self.K2_GetActorLocation`))
  (set `self.StartLocation` _returnvalue)
  (set `self.Target Location` (+ _returnvalue (* (`self.GetActorUpVector`) 500.0)))
  (`/Engine/EditorBlueprintResources/StandardMacros.FlipFlop` :!label _label
    (:`A`
      (bind (_direction _output) (`Timeline|타임라인_0` :!label _label_2)
        (:`Update`
          (`self.K2_SetActorLocation` (`KismetMathLibrary.VLerp` (`self.StartLocation`) (`self.Target Location`) _output)))
        (:`Finished`
          (goto _label))))
    (:`B`
      (goto _label_2 :!via `Reverse`))))

(fn `UserConstructionScript`)