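; BP_RotateCylinder is a rotating Stage2 hazard that ragdolls the player when its beam hits them.
; It turns by a fixed step every Tick, independent of delta time, and draws a red debug line between two inherited meshes.
; A Pawn-only line trace along that span detects hits and calls Ragdoll on BP_Player.
; Mesh collision is disabled on BeginPlay, so the trace alone handles detection.
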(event `self.ReceiveBeginPlay`
  (`PrimitiveComponent.SetCollisionEnabled` (`self.InheritMesh1`) "NoCollision")
  (`PrimitiveComponent.SetCollisionEnabled` (`self.InheritMesh2`) "NoCollision")
  (`PrimitiveComponent.SetCollisionEnabled` (`self.StaticMeshComponent`) "NoCollision"))

(event `self.ReceiveTick`
  (params (DeltaSeconds :type "Float (single-precision)"))
  (bind _returnvalue (`SceneComponent.K2_GetComponentLocation` (`self.InheritMesh2`)))
  (bind _returnvalue_2 (`SceneComponent.K2_GetComponentLocation` (`self.InheritMesh1`)))
  (`self.K2_AddActorWorldRotation` (struct :`Yaw` 1.0))
  (`KismetSystemLibrary.DrawDebugLine` _returnvalue_2 _returnvalue (struct :`R` 1.0 :`A` 1.0) 0.0 20.0)
  (bind (_outhit _returnvalue_3) (`KismetSystemLibrary.LineTraceSingleForObjects` :`Start` _returnvalue_2 :`End` _returnvalue :`ObjectTypes` (`|MakeArray` "ObjectTypeQuery3" :!type "EObjectTypeQuery Enum") :`DrawDebugType` "ForOneFrame"))
  (if _returnvalue_3
    (bind _asbp_player (cast `/Game/Player/BP_Player` (`.HitActor` (`GameplayStatics.BreakHitResult` _outhit))))
    (`/Game/Player/BP_Player.Ragdoll` _asbp_player)))

(fn `UserConstructionScript`)