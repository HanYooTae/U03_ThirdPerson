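; BP_ForwardLine2 is a Stage 2 laser-style line hazard that ragdolls the player on contact.
; On BeginPlay it caches every BP_ForwardCylinder in the level and uses the actors at indices 2 and 3 as endpoints, so the pairing depends on array order.
; Each Tick it draws a thick red debug line between them and traces for Pawns, calling Ragdoll on any BP_Player hit.
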(event `self.ReceiveBeginPlay`
  (bind _outactors (`GameplayStatics.GetAllActorsOfClass` "/Game/과제/Stage2/Cylinder/BP_ForwardCylinder.BP_ForwardCylinder_C"))
  (set `self.Cylinder` _outactors))

(event `self.ReceiveTick`
  (params (DeltaSeconds :type "Float (single-precision)"))
  (bind _cylinder (`self.Cylinder`))
  (bind _returnvalue (`self.K2_GetActorLocation` (`|GetArrayItem` _cylinder 2)))
  (bind _returnvalue_2 (`self.K2_GetActorLocation` (`|GetArrayItem` _cylinder 3)))
  (`KismetSystemLibrary.DrawDebugLine` _returnvalue _returnvalue_2 (struct :`R` 1.0 :`A` 1.0) 0.0 20.0)
  (bind (_outhit _returnvalue_3) (`KismetSystemLibrary.LineTraceSingleForObjects` _returnvalue _returnvalue_2 (`|MakeArray` "ObjectTypeQuery3" :!type "EObjectTypeQuery Enum") false (`self.Cylinder`) "ForOneFrame"))
  (if _returnvalue_3
    (bind _asbp_player (cast `/Game/Player/BP_Player` (`.HitActor` (`GameplayStatics.BreakHitResult` _outhit))))
    (`/Game/Player/BP_Player.Ragdoll` _asbp_player)))

(fn `UserConstructionScript`)