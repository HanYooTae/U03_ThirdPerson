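; BP_Enemy_AI is an enemy pawn Blueprint that shows debug-style name labels and feeds a patrol route to its patrol component.
; The construction script writes the pawn's display name to a PawnName text and copies its Path variable into PatrolComponent.
; BeginPlay runs the parent logic, then sets a ControllerName text to the display name of the possessing controller.
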(event `self.ReceiveBeginPlay`
  (`parent.ReceiveBeginPlay`)
  (`TextRenderComponent.K2_SetText` (`self.ControllerName`) (`KismetTextLibrary.Conv_StringToText` (`KismetSystemLibrary.GetDisplayName` (`self.GetController`)))))

(fn `UserConstructionScript`
  (`parent.UserConstructionScript`)
  (`TextRenderComponent.K2_SetText` (`self.PawnName`) (`KismetTextLibrary.Conv_StringToText` (`KismetSystemLibrary.GetDisplayName` self)))
  (set `/Game/Components/PatrolComponent.Path` (`self.Path`) (`self.PatrolComponent`)))