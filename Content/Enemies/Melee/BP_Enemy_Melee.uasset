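; BP_Enemy_Melee is a melee enemy that wields a great sword, extending a parent Blueprint's weapon equip logic.
; Attach and Detach move the GreatSword component between hand and holster sockets and toggle OnHand, with Attach also setting CombatType.
; Equipped and Unequipped call the parent, then set the great sword as current weapon or clear it.
; Several leftover CombatType and StateType setters are disconnected and never run.
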(event `self.ReceiveBeginPlay`
  (`parent.ReceiveBeginPlay`))

(event `self.Attach`
  (`parent.Attach`)
  (`self.K2_AttachToComponent` (`self.GreatSword`) (`self.Mesh`) "Hand_GreateSword" "KeepRelative" "KeepRelative" "KeepRelative" true)
  (set `self.bOnHand` true)
  (set `self.CombatType` "NewEnumerator1"))

(event `self.Detach`
  (`parent.Detach`)
  (`self.K2_AttachToComponent` (`self.GreatSword`) (`self.Mesh`) "Holster_GreateSword" "KeepRelative" "KeepRelative" "KeepRelative" true)
  (set `self.bOnHand` false))

(event `self.Equipped`
  (`parent.Equipped`)
  (bind _weapon (`self.SetCurrentWeapon` (`self.GreatSword`))))

(event `self.Unequipped`
  (`parent.Unequipped`)
  (bind _weapon (`self.SetCurrentWeapon` null)))

(fn `UserConstructionScript`
  (`parent.UserConstructionScript`))