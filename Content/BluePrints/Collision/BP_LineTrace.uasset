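; BP_LineTrace acts as a trip line between two vertex actors that ragdolls the player on contact.
; On BeginPlay it gathers every BP_Vertex in the level, then each Tick traces for Pawn objects between the first two in that array.
; The trace ignores the vertices and draws debug for one frame, and a hit on a BP_Player calls its Ragdoll function.
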(event `self.ReceiveBeginPlay`
  (bind _outactors (`GameplayStatics.GetAllActorsOfClass` "/Game/BluePrints/Collision/BP_Vertex.BP_Vertex_C"))
  (set `self.Vertices` _outactors))

(event `self.ReceiveTick`
  (params (DeltaSeconds :type "Float (single-precision)"))
  (bind _vertices (`self.Vertices`))
  (bind (_outhit _returnvalue) (`KismetSystemLibrary.LineTraceSingleForObjects` (`self.K2_GetActorLocation` (`|GetArrayItem` _vertices)) (`self.K2_GetActorLocation` (`|GetArrayItem` _vertices 1)) (`|MakeArray` "ObjectTypeQuery3" :!type "EObjectTypeQuery Enum") false (`self.Vertices`) "ForOneFrame"))
  (if _returnvalue
    (bind _asbp_player (cast `/Game/Player/BP_Player` (`.HitActor` (`GameplayStatics.BreakHitResult` _outhit))))
    (`/Game/Player/BP_Player.Ragdoll` _asbp_player)))

(fn `UserConstructionScript`)