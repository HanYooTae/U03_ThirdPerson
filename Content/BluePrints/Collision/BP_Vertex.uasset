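; BP_Vertex is an actor in the Collision folder that moves back and forth along its forward vector.
; On BeginPlay it stores its start location and a target a short distance ahead.
; A timeline lerps the actor between the two points without sweep, and its Finished output re-enters a FlipFlop that alternates Play and Reverse to keep the motion cycling.
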(event `self.ReceiveBeginPlay`
  (bind _returnvalue (`self.K2_GetActorLocation`))
  (set `self.StartLocation` _returnvalue)
  (set `self.Target Location` (+ _returnvalue (* (`self.GetActorForwardVector`) 50.0)))
  (`/Engine/EditorBlueprintResources/StandardMacros.FlipFlop` :!label _label
    (:`A`
      (bind (_direction _output) (`Timeline|Timeline` :!label _label_2)
        (:`Update`
          (`self.K2_SetActorLocation` (`KismetMathLibrary.VLerp` (`self.StartLocation`) (`self.Target Location`) _output)))
        (:`Finished`
          (goto _label))))
    (:`B`
      (goto _label_2 :!via `Reverse`))))

(fn `UserConstructionScript`)