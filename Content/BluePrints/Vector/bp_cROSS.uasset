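; Debug Blueprint that visualizes the cross product between actor A's forward vector and the vector from A to actor B.
; Each Tick it draws debug arrows from A for the A-to-B vector, scaled forward vector and cross result, using small getter functions.
; It also updates text displays with A-to-B (labeled "B Location"), the cross vector, and its dot with A's up vector, a signed left/right measure.
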(event `self.ReceiveTick`
  (params (DeltaSeconds :type "Float (single-precision)"))
  (bind _returnvalue (`self.Get_A_Location`))
  (bind _returnvalue_2 (`self.Get_A_Location`))
  (bind _returnvalue_3 (`KismetMathLibrary.Cross_VectorVector` (`self.Get_A_Forward_Vector`) (`self.Get_A_to_B_Vector`)))
  (`|ExecutionSequence`
    (:`then_0`
      (`KismetSystemLibrary.DrawDebugArrow` (`self.Get_A_Location`) (`self.Get_B_Location`) 0.0 (struct :`R` 1.0 :`A` 1.0) 0.0 2.0))
    (:`then_1`
      (`KismetSystemLibrary.DrawDebugArrow` _returnvalue (+ _returnvalue (* (`self.Get_A_Forward_Vector`) 300.0)) 0.0 (struct :`G` 1.0 :`A` 1.0) 0.0 2.0))
    (:`then_2`
      (`KismetSystemLibrary.DrawDebugArrow` _returnvalue_2 (+ _returnvalue_2 (`KismetMathLibrary.Cross_VectorVector` (`self.Get_A_Forward_Vector`) (`self.Get_A_to_B_Vector`))) 0.0 (struct :`B` 1.0 :`A` 1.0) 0.0 3.0))
    (:`then_3`
      (`|ExecutionSequence`
        (:`then_0`
          (`TextRenderComponent.K2_SetText` (`self.Print_B_Location`) (`KismetTextLibrary.Conv_StringToText` (`KismetStringLibrary.Concat_StrStr` "B Location : " (`KismetStringLibrary.Conv_VectorToString` (`self.Get_A_to_B_Vector`))))))
        (:`then_1`
          (`TextRenderComponent.K2_SetText` (`self.Cross_Result`) (`KismetTextLibrary.Conv_StringToText` (`KismetStringLibrary.Concat_StrStr` "Cross : " (`KismetStringLibrary.Conv_VectorToString` _returnvalue_3)))))
        (:`then_2`
          (`TextRenderComponent.K2_SetText` (`self.Dot_Result`) (`KismetTextLibrary.Conv_StringToText` (`KismetStringLibrary.Concat_StrStr` "Dot : " (`KismetStringLibrary.Conv_DoubleToString` (`KismetMathLibrary.Dot_VectorVector` _returnvalue_3 (`self.GetActorUpVector` (`self.A`))))))))))))

(fn `Get_A_Forward_Vector`
  (returns (ReturnValue :type "Vector Structure"))
  (return (`self.GetActorForwardVector` (`self.A`))))

(fn `Get_A_Location`
  (returns (ReturnValue :type "Vector Structure"))
  (return (`self.K2_GetActorLocation` (`self.A`))))

(fn `Get_A_to_B_Vector`
  (returns (ReturnValue :type "Vector Structure"))
  (return (- (`self.Get_B_Location`) (`self.Get_A_Location`))))

(fn `Get_B_Location`
  (returns (ReturnValue :type "Vector Structure"))
  (return (`self.K2_GetActorLocation` (`self.B`))))

(fn `UserConstructionScript`)