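; BP_Dot is a dot product visualizer that labels each StaticMeshActor tagged DotTarget with its dot product relative to this actor.
; On BeginPlay it gathers the targets and adds a centered red text render component above each, stored in a parallel array.
; PrintDotResult then writes each GetDotProductTo value into the matching label, running once at startup rather than on tick.
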(event `self.ReceiveBeginPlay`
  (bind _outactors (`GameplayStatics.GetAllActorsOfClassWithTag` "/Script/Engine.StaticMeshActor" "DotTarget"))
  (bind _output_get (set `self.DotTargets` _outactors))
  (for _array_element _output_get
    (bind _returnvalue (`AddComponent|NODE_AddTextRenderComponent-0` :`self` _array_element :`RelativeTransform` (`KismetMathLibrary.MakeTransform` (0.0 0.0 70.0) (struct :`Pitch` 90.0 :`Yaw` 180.0))))
    (`TextRenderComponent.SetHorizontalAlignment` _returnvalue "EHTA_Center")
    (`TextRenderComponent.SetTextRenderColor` _returnvalue (make `Color` 0 0 1 1))
    (`KismetArrayLibrary.Array_Add` (`self.TextRenders`) _returnvalue))
  (`self.PrintDotResult`))

(event `PrintDotResult`
  (for (_array_element _array_index) (`self.DotTargets`)
    (`TextRenderComponent.K2_SetText` (`|GetArrayItem` (`self.TextRenders`) _array_index) (`KismetTextLibrary.Conv_DoubleToText` (`self.GetDotProductTo` _array_element) "HalfToEven"))))

(fn `UserConstructionScript`)